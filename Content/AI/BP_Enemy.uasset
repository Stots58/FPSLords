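; BP_Enemy is an AI enemy that roams between target points and chases the first-person player.
; It loops moving to random reachable spots near random TargetPoints, switching to a faster chase on perception updates and resuming the slower roam when the player is forgotten.
; Reaching the player turns on physics simulation for the enemy's own mesh.
; Damage goes through BPCHealth, and on death Spawner spawns a replacement before the actor is destroyed.
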(event OnTargetPerceptionForgotten(AIPerception)
  (params (Actor :type Actor%20Object%20Reference))
  ;[0.15 0.15 0.15 0.5] AI Pathing Walk
  (Utilities|Casting|CastToBP_FirstPersonCharacter Actor
    (:then
      (Variables|/Script/Engine.CharacterMovementComponent|SetMaxWalkSpeed (Variables|Character|GetCharacterMovement) 3e+02)
      (CallFunction|UpdateAITarget))
    (:CastFailed
      _))
  (Development|PrintString "Hello"))

(event OnTargetPerceptionUpdated(AIPerception)
  (params (Actor :type Actor%20Object%20Reference) (Stimulus :type AI%20Stimulus%20Structure))
  ;[0.15 0.15 0.15 0.5] AI Chase & Death 'n respawn
  (bind _asbp_first_person_character (Utilities|Casting|CastToBP_FirstPersonCharacter Actor))
  (Variables|/Script/Engine.CharacterMovementComponent|SetMaxWalkSpeed (Variables|Character|GetCharacterMovement) 5e+02)
  (AI|AIMoveTo self "0, 0, 0" _asbp_first_person_character 5.0 false
    (:OnSuccess
      (Physics|SetSimulatePhysics (Variables|Character|GetMesh) true))))

(event Custom|Update%20AI%20Target
  ;[0.15 0.15 0.15 0.5] AI Pathing
  (AI|AIMoveTo self (.RandomLocation (AI|Navigation|GetRandomReachablePointinRadius (Transformation|GetActorLocation (.OutItem (Utilities|Array|Random (Variables|Default|GetOut%20Actors)))) 2.5e+02 0 0)) 0 5.0 false :!label _label
    (:OnSuccess
      (Utilities|FlowControl|Delay 1.5)
      (goto _label))))

(event Custom|OnTargetPerceptionForgotten_Event
  (params (Actor :type Actor%20Object%20Reference))
  ;[0.15 0.15 0.15 0.5] AI Pathing
  (Development|PrintString (Utilities|String|ToString(Text) (Utilities|Text|FormatText "AI Forget this {actor}" Actor))))

(event EventBeginPlay
  ;[0.15 0.15 0.15 0.5] AI Pathing
  (EventDispatchers|AssignOnTargetPerceptionForgotten (Variables|Default|GetAIPerception) (delegate Custom|OnTargetPerceptionForgotten_Event))
  (bind _outactors (Actor|GetAllActorsOfClass "/Script/Engine.TargetPoint"))
  (Variables|Default|SetOut%20Actors _outactors)
  (CallFunction|UpdateAITarget))

(event Game|Damage|EventAnyDamage
  (params (Damage :type Float%20%28single-precision%29) (DamageType :type Damage%20Type%20Object%20Reference) (InstigatedBy :type Controller%20Object%20Reference) (DamageCauser :type Actor%20Object%20Reference))
  (bind _isdead (Default|DamageTaken1 (Variables|Default|GetBPC_Health) Damage))
  (if _isdead
    (Default|SpawnEnemy (Variables|Default|Getspawner))
    (Actor|DestroyActor)))

(fn ConstructionScript)